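; BP_LevelChunk is a level segment that spawns and clears copies of itself as the player moves through it, producing a repeating level.
; The Spawn trigger creates the next chunk at a fixed offset along negative X when BP_Player overlaps it, with the Destroy flag preventing repeat spawns.
; The Kill trigger destroys every other BP_LevelChunk when the player overlaps it, leaving only the current one.
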(event OnComponentBeginOverlap(spawn)
  (params (OverlappedComponent :type Primitive%20Component%20Object%20Reference) (OtherActor :type Actor%20Object%20Reference) (OtherComp :type Primitive%20Component%20Object%20Reference) (OtherBodyIndex :type Integer) (bFromSweep :type Boolean) (SweepResult :type Hit%20Result%20Structure%20%28by%20ref%29))
  (bind _returnvalue (Transformation|GetActorLocation))
  (if (and (== (Utilities|GetClass OtherActor) "/Game/Blueprints/BP_Player.BP_Player_C") (not (Variables|Default|Getdestroy)))
    (Game|SpawnActorfromClass "BP_LevelChunk_C" (Math|Transform|MakeTransform (Math|Vector|MakeVector (- (.x _returnvalue) 1.55e+04) (.y _returnvalue) (.z _returnvalue)) "0, 0, 0" "1.000000,1.000000,1.000000") "AlwaysSpawn" "MultiplyWithRoot" 0 0 0 0)
    (Variables|Default|Setdestroy true)))

(event OnComponentBeginOverlap(kill)
  (params (OverlappedComponent :type Primitive%20Component%20Object%20Reference) (OtherActor :type Actor%20Object%20Reference) (OtherComp :type Primitive%20Component%20Object%20Reference) (OtherBodyIndex :type Integer) (bFromSweep :type Boolean) (SweepResult :type Hit%20Result%20Structure%20%28by%20ref%29))
  (if (== (Utilities|GetClass OtherActor) "/Game/Blueprints/BP_Player.BP_Player_C")
    (bind _outactors (Actor|GetAllActorsOfClass "BP_LevelChunk_C"))
    (for _array_element _outactors
      (if (!= _array_element self)
        (Actor|DestroyActor _array_element)))))

(event EventBeginPlay)

(event Collision|EventActorBeginOverlap
  (params (OtherActor :type Actor%20Object%20Reference)))

(fn ConstructionScript)